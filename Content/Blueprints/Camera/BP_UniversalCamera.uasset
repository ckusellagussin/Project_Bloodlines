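; BP_UniversalCamera is a player-controlled camera that spawns a top-down character at its location and follows it from BeginPlay.
; BeginPlay also adds the Enhanced Input mapping context and shows the mouse cursor.
; Y toggles following and changes the target offset, while middle mouse holds screen sliding.
; Zoom uses Enhanced Input, while movement and yaw use legacy axis events, all forwarding to camera functions defined outside this graph.
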(event Input|EnhancedActionEvents|EnhancedInputActionIA_Zoom
  (params (ActionValue :type Float%20%28double-precision%29) (ElapsedSeconds :type Float%20%28double-precision%29) (TriggeredSeconds :type Float%20%28double-precision%29) (InputAction :type Input%20Action%20Object%20Reference :default "/Game/Utilities/IA_Zoom.IA_Zoom"))
  (:Triggered
    (Class|UniversalCamera|Zoomin ActionValue 1.0)))

(event EventBeginPlay
  (Utilities|FlowControl|Sequence
    (:then_0
      (Input|AddMappingContext (PlayerController|LocalPlayerSubsystems|GetEnhancedInputLocalPlayerSubsystem (Game|GetPlayerController 0)) "/Game/Utilities/InputMappingContext.InputMappingContext" 0 "(bIgnoreAllPressedKeysUntilRelease=True,bForceImmediately=False)")
      (bind _returnvalue (Game|SpawnActorfromClass "/Game/Blueprints/Character/BP_TopDownCharacter.BP_TopDownCharacter_C" (Math|Transform|MakeTransform (Transformation|GetActorLocation) "0, 0, 0" "1.000000,1.000000,1.000000") "Undefined" "MultiplyWithRoot" 0 self))
      (bind _output_get (Variables|Default|SetTopDownCharacter _returnvalue))
      (Class|UniversalCamera|FollowTarget :TargetSettings (Class|UniversalCamera|UseActor _output_get)))
    (:then_1
      (Variables|/Script/Engine.PlayerController|SetbShowMouseCursor (Game|GetPlayerController 0) true))))

(event Input|AxisEvents|InputAxisMoveForward
  (params (AxisValue :type Float%20%28single-precision%29))
  (Class|UniversalCamera|MoveForward AxisValue 1.0 false false))

(event Input|AxisEvents|InputAxisRotateYaw
  (params (AxisValue :type Float%20%28single-precision%29))
  (Class|UniversalCamera|RotateYaw AxisValue 1.0 false))

(event Input|AxisEvents|InputAxisMoveRight
  (params (AxisValue :type Float%20%28single-precision%29))
  (Class|UniversalCamera|MoveRight AxisValue 1.0 false false))

(event Input|MouseEvents|MiddleMouseButton
  (params (Key :type Key%20Structure :default "None"))
  (:Pressed
    (Class|UniversalCamera|ToggleScreenSliding true))
  (:Released
    (Class|UniversalCamera|ToggleScreenSliding false)))

(event Input|KeyboardEvents|Y
  (params (Key :type Key%20Structure :default "None"))
  (:Pressed
    (if (Class|UniversalCamera|IsFollowingAnyActor)
      (Class|UniversalCamera|SetDesiredTargetOffset "0, 0, 0" false false)
      (Class|UniversalCamera|StopFollowing false)
      (else
        (Class|UniversalCamera|SetDesiredTargetOffset "0.000000,0.000000,-220.000000" false false)
        (Class|UniversalCamera|FollowTarget :TargetSettings (Class|UniversalCamera|UseActor (Variables|Default|GetTopDownCharacter)))))))

(fn ConstructionScript)