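; BP_Door is an interactable door that toggles between Open and Close.
; Interact flips the current context menu option and plays or reverses the Move timeline, which lerps the Scene component's yaw between 0 and 90 degrees.
; The timeline update feeds the component's relative location X and Y into roll and pitch.
; Getter functions expose the current option, description and object name.
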(event EventInteract
  (bind _scene (Variables|Default|GetScene))
  (bind _relativelocation (Variables|/Script/Engine.SceneComponent|GetRelativeLocation _scene))
  (switch Utilities|FlowControl|Switch|SwitchonE_ContextMenuOptions (Variables|Default|GetCurrent%20Context%20Menu%20Option)
    (:NewEnumerator0
      (Variables|Default|SetCurrent%20Context%20Menu%20Option "NewEnumerator1")
      (bind _alpha (Timeline|Move Play)
        (:Update
          (Transformation|SetRelativeRotation _scene (Math|Rotator|MakeRotator (.x _relativelocation) (.y _relativelocation) (Math|Float|Lerp 0.0 9e+01 _alpha)) false false))))
    (:NewEnumerator1
      (Variables|Default|SetCurrent%20Context%20Menu%20Option "NewEnumerator0")
      (Timeline|Move Reverse))))

(fn ConstructionScript)

(fn GetContextOptions
  (return (Variables|Default|GetCurrent%20Context%20Menu%20Option)))

(fn GetDescription
  (return (Variables|Default|GetDescription)))

(fn GetObjectName
  (return (Variables|Default|GetName)))